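; Player ship Blueprint for a scrolling shooter, handling movement, firing, death and stage clear.
; After Space release dismisses the opening Cube, Tick scrolls the actor along X unless ScStop is set, while WASD offsets the ship mesh inside it.
; Space fires BP_J_tama with a short cooldown; enemy or bullet hits show an explosion, then restart via myGamemode.
; Trigger volumes wake sleeping BP_teki enemies and destroy passing enemies and bullets; EV_clear shows clear visuals, then restarts.
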(event `InputAction|AC_A`
  (params (Key :type "Key Structure"))
  (:`Pressed`
    (set `self.jikiY` -2.0))
  (:`Released`
    (set `self.jikiY` 0.0 :!label _label)))

(event `InputAction|AC_D`
  (params (Key :type "Key Structure"))
  (:`Pressed`
    (set `self.jikiY` 2.0))
  (:`Released`
    (goto _label)))

(event `InputAction|AC_S`
  (params (Key :type "Key Structure"))
  (:`Pressed`
    (set `self.jikiX` -2.0))
  (:`Released`
    (set `self.jikiX` 0.0 :!label _label_2)))

(event `InputAction|AC_W`
  (params (Key :type "Key Structure"))
  (:`Pressed`
    (set `self.jikiX` 2.0))
  (:`Released`
    (goto _label_2)))

(event `Key|SpaceBar`
  (params (Key :type "Key Structure"))
  (:`Pressed`
    (if (`self.uteru`)
      (`|SpawnActorFromClass` "/Game/BP/BP_J_tama.BP_J_tama_C" (`SceneComponent.K2_GetComponentToWorld` (`self.Arrow`)) "Undefined" "OverrideRootScale" null null)
      (set `self.uteru` false)
      (`KismetSystemLibrary.Delay` 0.2)
      (if (`SceneComponent.bVisible` (`self.StaticMesh`))
        (set `self.uteru` true))))
  (:`Released`
    (if (`self.gameop`)
      (set `self.gameop` false)
      (`SceneComponent.SetVisibility` (`self.Cube`) false true))))

(event `self.ReceiveTick`
  (params (DeltaSeconds :type "Float (single-precision)"))
  (bind _staticmesh (`self.StaticMesh`))
  (bind (_relativelocation_x _relativelocation_y _relativelocation_z) (`KismetMathLibrary.BreakVector` (`SceneComponent.RelativeLocation` _staticmesh)))
  (if (not (`self.gameop`))
    (if (not (`self.sc_stop`))
      (`self.K2_SetActorLocation` (+ (`self.K2_GetActorLocation`) (0.2 0.0 0.0))))
    (if (`self.uteru`)
      (`SceneComponent.K2_SetRelativeLocation` _staticmesh (`KismetMathLibrary.MakeVector` (+ _relativelocation_x (`self.jikiX`)) (+ _relativelocation_y (`self.jikiY`)) _relativelocation_z) false false))))

(event `self.Box.OnComponentBeginOverlap`
  (params (OverlappedComponent :type "PrimitiveComponent Object Reference") (OtherActor :type "Actor Object Reference") (OtherComp :type "PrimitiveComponent Object Reference") (OtherBodyIndex :type Integer) (bFromSweep :type Boolean) (SweepResult :type "HitResult Structure (by ref)"))
  (bind _bakuhu (`self.bakuhu`))
  (bind _asbp_teki (cast `/Game/BP/BP_teki` OtherActor)
    (:`then`
      (`self.K2_DestroyActor` _asbp_teki))
    (:`CastFailed`
      (bind _asbp_t_tama (cast `/Game/BP/BP_T_tama` OtherActor))
      (`self.K2_DestroyActor` _asbp_t_tama)))
  (set `self.uteru` false)
  (`PrimitiveComponent.SetCollisionEnabled` (`self.Box`) "NoCollision")
  (`SceneComponent.SetVisibility` (`self.StaticMesh`) false false)
  (`SceneComponent.SetVisibility` _bakuhu true false)
  (`KismetSystemLibrary.Delay` 10.0)
  (`SceneComponent.SetVisibility` _bakuhu false false)
  (`KismetSystemLibrary.Delay` 5.0)
  (bind _asmy_gamemode (cast `/Game/BP/Enum/myGamemode` (`GameplayStatics.GetGameMode`)))
  (`GameMode.RestartGame` _asmy_gamemode))

(event `self.okiru.OnComponentBeginOverlap`
  (params (OverlappedComponent :type "PrimitiveComponent Object Reference") (OtherActor :type "Actor Object Reference") (OtherComp :type "PrimitiveComponent Object Reference") (OtherBodyIndex :type Integer) (bFromSweep :type Boolean) (SweepResult :type "HitResult Structure (by ref)"))
  (bind _asbp_teki (cast `/Game/BP/BP_teki` OtherActor))
  (if (`/Game/BP/BP_teki.SLEEP` _asbp_teki)
    (set `/Game/BP/BP_teki.SLEEP` false _asbp_teki)
    (`/Game/BP/BP_teki.okita` _asbp_teki)))

(event `self.destro.OnComponentBeginOverlap`
  (params (OverlappedComponent :type "PrimitiveComponent Object Reference") (OtherActor :type "Actor Object Reference") (OtherComp :type "PrimitiveComponent Object Reference") (OtherBodyIndex :type Integer) (bFromSweep :type Boolean) (SweepResult :type "HitResult Structure (by ref)"))
  (bind _asbp_teki (cast `/Game/BP/BP_teki` OtherActor)
    (:`then`
      (`self.K2_DestroyActor` _asbp_teki))
    (:`CastFailed`
      (bind _asbp_t_tama (cast `/Game/BP/BP_T_tama` OtherActor))
      (`self.K2_DestroyActor` _asbp_t_tama))))

(event `EV_clear`
  (`SceneComponent.SetVisibility` (`self.Cube`) true false)
  (`SceneComponent.SetVisibility` (`self.TextRender2`) true false)
  (`KismetSystemLibrary.Delay` 10.0)
  (bind _asmy_gamemode (cast `/Game/BP/Enum/myGamemode` (`GameplayStatics.GetGameMode`)))
  (`GameMode.RestartGame` _asmy_gamemode))

(fn `UserConstructionScript`)