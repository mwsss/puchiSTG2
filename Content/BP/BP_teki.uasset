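; BP_teki is a configurable shooter enemy whose type (SYURUI) covers small, mid-size, boss and ground variants, with its mesh set at construction.
; The okita event starts a repeating delayed fire loop that spawns 1- to 5-way bullets, optionally yaw-aimed at the player.
; Small and mid-size types drift along -X unless asleep.
; Player bullets drain HP until death; bosses also set the player's ScStop and call EVClear.
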(event `okita`
  (if (`self.TAMA`)
    (bind _asbp_jiki (cast `/Game/BP/BP_jiki` (`GameplayStatics.GetPlayerPawn` 0)))
    (set `self.OB_jiki` _asbp_jiki)
    (switch `/Game/BP/Enum/EN_syurui` (`self.SYURUI`)
      (:`NewEnumerator0`
        _)
      (:`NewEnumerator1`
        _)
      (:`NewEnumerator2`
        (`KismetSystemLibrary.Delay` 17.0)
        (set `/Game/BP/BP_jiki.sc_stop` true _asbp_jiki))
      (:`NewEnumerator3`
        _))
    (`self.tamautu`)))

(event `tamautu`
  (bind _arrow (`self.Arrow`))
  (bind (_returnvalue_roll _returnvalue_pitch _returnvalue_yaw) (`KismetMathLibrary.BreakRotator` (`KismetMathLibrary.FindLookAtRotation` (`SceneComponent.K2_GetComponentLocation` _arrow) (`SceneComponent.K2_GetComponentLocation` (`/Game/BP/BP_jiki.Box` (`self.OB_jiki`))))))
  (`KismetSystemLibrary.Delay` 2.0)
  (if (`self.TAMA`)
    (if (`self.NERAI`)
      (`SceneComponent.K2_SetRelativeRotation` _arrow (`KismetMathLibrary.MakeRotator` 0.0 0.0 _returnvalue_yaw) false true))
    (switch `/Game/BP/Enum/EN_tway` (`self.WAY`)
      (:`NewEnumerator0`
        (`|SpawnActorFromClass` "/Game/BP/BP_T_tama.BP_T_tama_C" (`SceneComponent.K2_GetComponentToWorld` (`self.Arrow`)) "Undefined" "OverrideRootScale" null null)
        (`self.tamautu` :!label _label))
      (:`NewEnumerator4`
        (`|SpawnActorFromClass` "/Game/BP/BP_T_tama.BP_T_tama_C" (`SceneComponent.K2_GetComponentToWorld` (`self.Arrow1`)) "Undefined" "OverrideRootScale" null null)
        (`|SpawnActorFromClass` "/Game/BP/BP_T_tama.BP_T_tama_C" (`SceneComponent.K2_GetComponentToWorld` (`self.Arrow2`)) "Undefined" "OverrideRootScale" null null)
        (goto _label))
      (:`NewEnumerator1`
        (`|SpawnActorFromClass` "/Game/BP/BP_T_tama.BP_T_tama_C" (`SceneComponent.K2_GetComponentToWorld` (`self.Arrow`)) "Undefined" "OverrideRootScale" null null)
        (`|SpawnActorFromClass` "/Game/BP/BP_T_tama.BP_T_tama_C" (`SceneComponent.K2_GetComponentToWorld` (`self.Arrow1`)) "Undefined" "OverrideRootScale" null null)
        (`|SpawnActorFromClass` "/Game/BP/BP_T_tama.BP_T_tama_C" (`SceneComponent.K2_GetComponentToWorld` (`self.Arrow2`)) "Undefined" "OverrideRootScale" null null)
        (goto _label))
      (:`NewEnumerator2`
        (`|SpawnActorFromClass` "/Game/BP/BP_T_tama.BP_T_tama_C" (`SceneComponent.K2_GetComponentToWorld` (`self.Arrow1`)) "Undefined" "OverrideRootScale" null null)
        (`|SpawnActorFromClass` "/Game/BP/BP_T_tama.BP_T_tama_C" (`SceneComponent.K2_GetComponentToWorld` (`self.Arrow2`)) "Undefined" "OverrideRootScale" null null)
        (`|SpawnActorFromClass` "/Game/BP/BP_T_tama.BP_T_tama_C" (`SceneComponent.K2_GetComponentToWorld` (`self.Arrow3`)) "Undefined" "OverrideRootScale" null null)
        (`|SpawnActorFromClass` "/Game/BP/BP_T_tama.BP_T_tama_C" (`SceneComponent.K2_GetComponentToWorld` (`self.Arrow4`)) "Undefined" "OverrideRootScale" null null)
        (`self.tamautu` :!label _label_2))
      (:`NewEnumerator3`
        (`|SpawnActorFromClass` "/Game/BP/BP_T_tama.BP_T_tama_C" (`SceneComponent.K2_GetComponentToWorld` (`self.Arrow`)) "Undefined" "OverrideRootScale" null null)
        (`|SpawnActorFromClass` "/Game/BP/BP_T_tama.BP_T_tama_C" (`SceneComponent.K2_GetComponentToWorld` (`self.Arrow1`)) "Undefined" "OverrideRootScale" null null)
        (`|SpawnActorFromClass` "/Game/BP/BP_T_tama.BP_T_tama_C" (`SceneComponent.K2_GetComponentToWorld` (`self.Arrow2`)) "Undefined" "OverrideRootScale" null null)
        (`|SpawnActorFromClass` "/Game/BP/BP_T_tama.BP_T_tama_C" (`SceneComponent.K2_GetComponentToWorld` (`self.Arrow3`)) "Undefined" "OverrideRootScale" null null)
        (`|SpawnActorFromClass` "/Game/BP/BP_T_tama.BP_T_tama_C" (`SceneComponent.K2_GetComponentToWorld` (`self.Arrow4`)) "Undefined" "OverrideRootScale" null null)
        (goto _label_2)))))

(event `self.ReceiveTick`
  (params (DeltaSeconds :type "Float (single-precision)"))
  (bind _returnvalue (`self.K2_GetActorLocation`))
  (if (not (`self.SLEEP`))
    (switch `/Game/BP/Enum/EN_syurui` (`self.SYURUI`)
      (:`NewEnumerator0`
        (`self.K2_SetActorLocation` (+ _returnvalue (-0.4 0.0 0.0))))
      (:`NewEnumerator1`
        (`self.K2_SetActorLocation` (+ _returnvalue (-0.15 0.0 0.0)))))))

(event `self.Box.OnComponentBeginOverlap`
  (params (OverlappedComponent :type "PrimitiveComponent Object Reference") (OtherActor :type "Actor Object Reference") (OtherComp :type "PrimitiveComponent Object Reference") (OtherBodyIndex :type Integer) (bFromSweep :type Boolean) (SweepResult :type "HitResult Structure (by ref)"))
  (bind _staticmesh1 (`self.StaticMesh1`))
  (bind _asbp_j_tama (cast `/Game/BP/BP_J_tama` OtherActor))
  (`self.K2_DestroyActor` _asbp_j_tama)
  (bind _output_get (set `self.HP` (- (`self.HP`) 1)))
  (if (< _output_get 1)
    (set `self.TAMA` false)
    (`PrimitiveComponent.SetCollisionEnabled` (`self.Box`) "NoCollision")
    (`SceneComponent.SetVisibility` (`self.StaticMesh`) false false)
    (`SceneComponent.SetVisibility` _staticmesh1 true false)
    (`KismetSystemLibrary.Delay` 3.0)
    (`SceneComponent.SetVisibility` _staticmesh1 false false)
    (`self.K2_DestroyActor`)
    (switch `/Game/BP/Enum/EN_syurui` (`self.SYURUI`)
      (:`NewEnumerator2`
        (bind _asbp_jiki (cast `/Game/BP/BP_jiki` (`GameplayStatics.GetPlayerPawn` 0)))
        (`/Game/BP/BP_jiki.EV_clear` _asbp_jiki)))))

(fn `UserConstructionScript`
  (`StaticMeshComponent.SetStaticMesh` (`self.StaticMesh`) (`self.MODERU`)))